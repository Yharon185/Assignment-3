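; BP_Projectile is a projectile that damages a designated target actor and leaves an explosion behind, apparently for a spider attack.
; Its collision component ignores the owner, applies damage only when the overlapped actor is the target, and calls OnHit to destroy the projectile on any other overlap too.
; A destroy delegate bound at BeginPlay spawns BP_Spider_ProjectileExplosion at the projectile's transform.
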(event OnComponentBeginOverlap(DamageCollision)
  (params (OverlappedComponent :type Primitive%20Component%20Object%20Reference) (OtherActor :type Actor%20Object%20Reference) (OtherComp :type Primitive%20Component%20Object%20Reference) (OtherBodyIndex :type Integer) (bFromSweep :type Boolean) (SweepResult :type Hit%20Result%20Structure%20%28by%20ref%29))
  (if (!= OtherActor (Components|GetOwner))
    (Utilities|FlowControl|Sequence
      (:then_0
        (if (== OtherActor (Variables|Default|GetTargetActor))
          (Game|Damage|ApplyDamage OtherActor (Variables|Default|GetDamage) 0 (Components|GetOwner))))
      (:then_1
        (CallFunction|OnHit)))))

(event EventBeginPlay
  (Game|BindEventtoOnDestroyed (EventDispatchers|CreateEvent :!event OnProjectileDestroyed)))

(fn ConstructionScript)

(fn OnHit
  (Actor|DestroyActor))

(fn OnProjectileDestroyed
  (params (DestroyedActor :type Actor%20Object%20Reference))
  (Game|SpawnActorfromClass "/Game/MyContent/Enemies/BP_Spider_ProjectileExplosion.BP_Spider_ProjectileExplosion_C" (Math|Transform|MakeTransform (Transformation|GetActorLocation) (Transformation|GetActorRotation) (Transformation|GetActorScale3D)) "Undefined" "MultiplyWithRoot" 0 0))