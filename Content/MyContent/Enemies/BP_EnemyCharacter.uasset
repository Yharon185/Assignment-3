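; BP_EnemyCharacter is a melee enemy with level-scaled health and XP reward that registers with and alerts its assigned camp.
; Attacks play random montages with motion warping toward the target, while helpers toggle weapon damage and Tick-driven target facing.
; Hits subtract health equal to the enemy's level, ignoring incoming damage, then turn it toward the causer.
; Survivors hit-react and interrupt their AI controller; death awards XP, disables collision and despawns on a timer.
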(event OnDamaged(BP_AC_Stats)
  (params (Damage :type Float%20%28double-precision%29)))

(event EventTick
  (params (DeltaSeconds :type Float%20%28single-precision%29))
  (CallFunction|HandleFaceTarget))

(event EventBeginPlay
  (Game|BindEventtoOnDestroyed (EventDispatchers|CreateEvent :!event Destroyed))
  (Utilities|FlowControl|Sequence
    (:then_0
      (CallFunction|InitialiseStats))
    (:then_1
      (bind _assignedcamp (Variables|Default|GetAssignedCamp)
        (:then
          (Default|AddEnemy _assignedcamp self))
        (:else)))))

(event Game|Damage|EventAnyDamage
  (params (Damage :type Float%20%28single-precision%29) (DamageType :type Damage%20Type%20Object%20Reference) (InstigatedBy :type Controller%20Object%20Reference) (DamageCauser :type Actor%20Object%20Reference))
  (CallFunction|OnTakeDamage (* (Variables|/Game/MyContent/Core/BP_AC_Stats.BP_AC_Stats_C|GetLevel (Variables|Default|GetBP_AC_Stats)) (+ (* Damage 0.0) 1.0)) DamageCauser))

(fn ConstructionScript
  (Actor|SetOwner (Variables|/Script/Engine.ChildActorComponent|GetChildActor (Variables|Default|GetWeaponActor)) self)
  (Variables|Default|SetMinMaxHealth (Variables|/Game/MyContent/Core/BP_AC_Stats.BP_AC_Stats_C|GetMaxHealth (Variables|Default|GetBP_AC_Stats))))

(fn OnTakeDamage
  (params (Amount :type Float%20%28double-precision%29) (DamageCauser :type Actor%20Object%20Reference))
  (Default|DamageHealth (Variables|Default|GetBP_AC_Stats) Amount)
  (Transformation|SetActorRotation (Math|Rotator|MakeRotator 0.0 0.0 (.yaw (Math|Rotator|FindLookatRotation (Transformation|GetActorLocation) (Transformation|GetActorLocation DamageCauser)))))
  (if (CallFunction|IsAlive)
    (CallFunction|PlayHitReact)
    (CallFunction|EnableHealthWidget true)
    (else
      (CallFunction|Death)
      (CallFunction|EnableHealthWidget false))))

(fn Death
  (bind _despawntimer (Variables|Default|GetDespawnTimer))
  (bind _mesh (Variables|Character|GetMesh))
  (bind _returnvalue (Components|SkeletalMesh|GetAnimInstance _mesh))
  (CallFunction|GivePlayerXP)
  (Variables|Actor|SetbCanBeDamaged false)
  (CallFunction|EnableFaceTarget false)
  (CallFunction|DeactivateDamage)
  (Animation|Montage|MontageStop _returnvalue 0.0 (Animation|Montage|GetCurrentActiveMontage _returnvalue))
  (Collision|SetCollisionEnabled (Variables|Collision|GetCapsuleComponent) "NoCollision")
  (CallFunction|InterruptEnemy (+ _despawntimer 1.0))
  (Actor|SetLifeSpan _despawntimer)
  (Default|CallOnDeath))

(fn IsAlive
  (return (> (Variables|/Game/MyContent/Core/BP_AC_Stats.BP_AC_Stats_C|GetHealth (Variables|Default|GetBP_AC_Stats)) 0.0)))

(fn Attack
  (if (Utilities|Array|IsNotEmpty (Variables|Default|GetAttackAnims))
    (Utilities|FlowControl|Sequence
      (:then_0
        (bind _targetactor (Variables|Default|GetTargetActor)
          (:then
            (Class|MotionWarpingComponent|AddorUpdateWarpTargetfromLocationandRotation (Variables|Default|GetMotionWarping) "AttackTarget" "0, 0, 0" (Math|Rotator|MakeRotator 0.0 0.0 (.yaw (Math|Rotator|FindLookatRotation (Transformation|GetActorLocation) (Transformation|GetActorLocation _targetactor))))))
          (:else
            (Class|MotionWarpingComponent|RemoveWarpTarget (Variables|Default|GetMotionWarping) "AttackTarget"))))
      (:then_1
        (bind _returnvalue (Animation|Montage|MontagePlay (Components|SkeletalMesh|GetAnimInstance (Variables|Character|GetMesh)) (.OutItem (Utilities|Array|Random (Variables|Default|GetAttackAnims))) 1.0 "Duration" 0.0 true))
        (return _returnvalue)))))

(fn ActivateDamage
  (bind _asbp_weapon (Utilities|Casting|CastToBP_Weapon (Variables|/Script/Engine.ChildActorComponent|GetChildActor (Variables|Default|GetWeaponActor))))
  (Default|ActivateDamage _asbp_weapon))

(fn DeactivateDamage
  (bind _asbp_weapon (Utilities|Casting|CastToBP_Weapon (Variables|/Script/Engine.ChildActorComponent|GetChildActor (Variables|Default|GetWeaponActor))))
  (Default|DeactivateDamage _asbp_weapon))

(fn PlayHitReact
  (bind _returnvalue (Animation|Montage|MontagePlay (Components|SkeletalMesh|GetAnimInstance (Variables|Character|GetMesh)) (Variables|Default|GetHitReactAnim) 1.0 "Duration" 0.0 true))
  (CallFunction|InterruptEnemy _returnvalue)
  (CallFunction|DeactivateDamage)
  (CallFunction|EnableFaceTarget false))

(fn SetEnemyTarget
  (params (TargetActor :type Actor%20Object%20Reference))
  (bind _output_get (Variables|Default|SetTargetActor TargetActor))
  (Default|AlertCamp (Variables|Default|GetAssignedCamp) self _output_get))

(fn SetAITarget
  (params (TargetActor :type Actor%20Object%20Reference))
  (bind _asbp_enemy_controller (Utilities|Casting|CastToBP_EnemyController (Pawn|GetController)))
  (Default|SetControlTarget _asbp_enemy_controller TargetActor))

(fn InterruptEnemy
  (params (Duration :type Float%20%28double-precision%29))
  (bind _asbp_enemy_controller (Utilities|Casting|CastToBP_EnemyController (Pawn|GetController)))
  (Default|InterruptAI _asbp_enemy_controller Duration))

(fn Destroyed
  (params (DestroyedActor :type Actor%20Object%20Reference)))

(fn HandleFaceTarget
  (if (Variables|Default|GetbFaceTarget)
    (Variables|Default|GetTargetActor
      (:then
        (Transformation|SetActorRotation (Math|Rotator|MakeRotator 0.0 0.0 (.yaw (Math|Interpolation|RInterpTo (Transformation|GetActorRotation) (Math|Rotator|FindLookatRotation (Transformation|GetActorLocation) (Transformation|GetActorLocation (Variables|Default|GetTargetActor))) (Utilities|Time|GetWorldDeltaSeconds) 1e+01)))))
      (:else))))

(fn EnableFaceTarget
  (params (Enable :type Boolean))
  (Variables|Default|SetbFaceTarget Enable))

(fn EnableHealthWidget
  (params (Enable :type Boolean))
  (Rendering|SetVisibility (Variables|Default|GetEnemyHealthHealthWidget) Enable false))

(fn SetEnemyLevel
  (params (Level :type Integer))
  (Default|SetLevel (Variables|Default|GetBP_AC_Stats) (Math|Conversions|ToFloat(Integer) Level))
  (Default|SetMaxHealth (Variables|Default|GetBP_AC_Stats) (* (Variables|/Game/MyContent/Core/BP_AC_Stats.BP_AC_Stats_C|GetLevel (Variables|Default|GetBP_AC_Stats)) (Variables|Default|GetMinMaxHealth)))
  (Default|SetHealth (Variables|Default|GetBP_AC_Stats) (Variables|/Game/MyContent/Core/BP_AC_Stats.BP_AC_Stats_C|GetMaxHealth (Variables|Default|GetBP_AC_Stats))))

(fn InitialiseStats
  (CallFunction|SetEnemyLevel (Math|Float|Truncate (Variables|/Game/MyContent/Core/BP_AC_Stats.BP_AC_Stats_C|GetLevel (Variables|Default|GetBP_AC_Stats))))
  (bind _asbp_uw_enemy_health (Utilities|Casting|CastToBP_UW_EnemyHealth (UserInterface|GetWidget (Variables|Default|GetEnemyHealthHealthWidget))))
  (Default|InitialiseHealth _asbp_uw_enemy_health (Variables|Default|GetBP_AC_Stats)))

(fn GivePlayerXP
  (bind _asbp_player_character (Utilities|Casting|CastToBP_PlayerCharacter (Game|GetPlayerCharacter 0)))
  (Default|AddXP (Variables|/Game/MyContent/Player/BP_PlayerCharacter.BP_PlayerCharacter_C|GetStats%20Component%20%28Player%29 _asbp_player_character) (* (Variables|Default|GetMinXPWorth) (Variables|/Game/MyContent/Core/BP_AC_Stats.BP_AC_Stats_C|GetLevel (Variables|Default|GetBP_AC_Stats)))))