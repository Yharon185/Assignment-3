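; BP_AC_Stats is a stats component that tracks health, max health and level, and reports whether health is above zero.
; Damage and heal functions route through SetHealth, which clamps to the 0–MaxHealth range.
; Each change fires a matching notification for health change, damage, heal or level change, with damage passing its amount.
; SetMaxHealth floors the maximum at zero but does not re-clamp current health.
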(event EventBeginPlay)

(event EventTick
  (params (DeltaSeconds :type Float%20%28single-precision%29)))

(fn SetHealth
  (params (Health :type Float%20%28double-precision%29))
  (Variables|Default|SetHealth (Math|Float|Clamp(Float) Health 0.0 (Variables|Default|GetMaxHealth)))
  (Default|CallOnHealthChange))

(fn SetMaxHealth
  (params (MaxHealth :type Float%20%28double-precision%29))
  (Variables|Default|SetMaxHealth (Math|Float|Max(Float) MaxHealth 0.0))
  (Default|CallOnHealthChange))

(fn DamageHealth
  (params (Amount :type Float%20%28double-precision%29))
  (CallFunction|SetHealth (- (Variables|Default|GetHealth) Amount))
  (Default|CallOnDamaged Amount))

(fn HealHealth
  (params (Amount :type Float%20%28double-precision%29))
  (CallFunction|SetHealth (+ (Variables|Default|GetHealth) Amount))
  (Default|CallOnHeal))

(fn SetLevel
  (params (Level :type Float%20%28double-precision%29))
  (Variables|Default|SetLevel Level)
  (Default|CallOnLevelChange))

(fn IsAlive
  (return (> (Variables|Default|GetHealth) 0.0)))