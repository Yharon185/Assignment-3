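; Player stats component that manages XP, levelling and stamina for BP_PlayerCharacter.
; AddXP triggers LevelUpEvent when the cap is reached, which levels up through the character's component reference, updates its displayed level, then scales MaxXP up.
; Stamina regenerates in a short-delay loop started at BeginPlay.
; StaminaUsage deducts a fixed cost and sets Tired, pausing regen through a retriggerable delay, while StaminaCheck tests a minimum threshold.
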(event Custom|StaminaDelay
  (Utilities|FlowControl|RetriggerableDelay 1.75 :!label _label)
  (Variables|Default|SetTired false)
  (CallFunction|StaminaRegen 0.3 :!label _label_2)
  (Utilities|FlowControl|Delay 0.01)
  (if (Variables|Default|GetTired)
    (goto _label)
    (else
      (goto _label_2))))

(event Custom|LevelUpEvent
  (bind _asbp_player_character (Utilities|Casting|CastToBP_PlayerCharacter (Game|GetPlayerCharacter 0)))
  (CallFunction|LevelUp (Variables|/Game/MyContent/Player/BP_PlayerCharacter.BP_PlayerCharacter_C|GetStats%20Component%20%28Player%29 _asbp_player_character))
  (bind _asbp_player_character_2 (Utilities|Casting|CastToBP_PlayerCharacter (Game|GetPlayerCharacter 0)))
  (Default|UpdatePlayerLevel _asbp_player_character_2 (Math|Float|Truncate (Variables|/Game/MyContent/Core/BP_AC_Stats.BP_AC_Stats_C|GetLevel (Variables|/Game/MyContent/Player/BP_PlayerCharacter.BP_PlayerCharacter_C|GetStats%20Component%20%28Player%29 _asbp_player_character))))
  (Development|PrintString (Utilities|String|ToString(Float) (Variables|/Game/MyContent/Core/BP_AC_Stats.BP_AC_Stats_C|GetLevel (Variables|/Game/MyContent/Player/BP_PlayerCharacter.BP_PlayerCharacter_C|GetStats%20Component%20%28Player%29 _asbp_player_character)))))

(event EventBeginPlay
  (Variables|Default|SetStamina (Variables|Default|GetMaxStamina))
  (Utilities|FlowControl|Delay 0.01)
  (Variables|Default|SetStamina (- (Variables|Default|GetStamina) 1.0))
  (CallFunction|StaminaRegen 0.3 :!label _label)
  (Utilities|FlowControl|Delay 0.01)
  (if (Variables|Default|GetTired)
    (Utilities|FlowControl|RetriggerableDelay 1.75)
    (Variables|Default|SetTired false)
    (goto _label)
    (else
      (goto _label))))

(fn SetXP
  (params (XP :type Float%20%28double-precision%29))
  (Variables|Default|SetXP (Math|Float|Max(Float) XP 0.0))
  (Default|CallOnXPChanged))

(fn SetMaxXP
  (params (MaxXP :type Float%20%28double-precision%29))
  (Variables|Default|SetMaxXP (Math|Float|Max(Float) MaxXP 0.0))
  (Default|CallOnXPChanged))

(fn AddXP
  (params (Amount :type Float%20%28double-precision%29))
  (CallFunction|SetXP (+ (Variables|Default|GetXP) Amount))
  (Default|CallOnXPAdded Amount)
  (if (>= (Variables|Default|GetXP) (Variables|Default|GetMaxXP))
    (CallFunction|LevelUpEvent)
    (Variables|Default|SetMaxXP (* (Variables|Default|GetMaxXP) 1.2))))

(fn LevelUp
  (Variables|Default|SetLevel (+ (Variables|Default|GetLevel) 1.0))
  (CallFunction|SetLevel (+ (Variables|Default|GetLevel) 1.0))
  (CallFunction|SetXP (- (Variables|Default|GetXP) (Variables|Default|GetMaxXP))))

(fn SetStamina
  (params (Stamina :type Float%20%28double-precision%29))
  (Variables|Default|SetStamina (Math|Float|Clamp(Float) Stamina 0.0 (Variables|Default|GetMaxStamina)))
  (Default|CallOnStaminaChange))

(fn SetMaxStamina
  (params (MaxStamina :type Float%20%28double-precision%29))
  (Variables|Default|SetMaxStamina (Math|Float|Max(Float) MaxStamina 0.0))
  (Default|CallOnStaminaChange))

(fn StaminaRegen
  (params (RegenAmount :type Float%20%28double-precision%29))
  (if (not (>= (Variables|Default|GetStamina) (Variables|Default|GetMaxStamina)))
    (Variables|Default|SetStamina (+ (Variables|Default|GetStamina) RegenAmount))
    (Default|CallOnStaminaChange)))

(fn StaminaUsage
  (Variables|Default|SetStamina (- (Variables|Default|GetStamina) 12.0))
  (Variables|Default|SetTired true)
  (Default|CallOnStaminaChange)
  (CallFunction|StaminaDelay))

(fn StaminaCheck
  (if (>= (Variables|Default|GetStamina) 9.0)
    (Variables|Default|SetStaminaCheckBool true)
    (if (Variables|Default|GetStaminaCheckBool)
      (return true))
    (else
      (Variables|Default|SetStaminaCheckBool false))))